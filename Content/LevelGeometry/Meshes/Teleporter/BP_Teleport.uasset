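; BP_Teleport is a teleporter that moves the first-person player character to a destination when it overlaps the collider.
; The overlap snaps the character to the TeleportLocation component's position and rotation, then optionally sets a Music_State_Group audio state from StateName when ChangeState is enabled.
; Each Tick, two rotator meshes counter-spin, speeding up as the player gets closer through a clamped distance-to-speed mapping.
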(event OnComponentBeginOverlap(TeleportCollider)
  (params (OverlappedComponent :type Primitive%20Component%20Object%20Reference) (OtherActor :type Actor%20Object%20Reference) (OtherComp :type Primitive%20Component%20Object%20Reference) (OtherBodyIndex :type Integer) (bFromSweep :type Boolean) (SweepResult :type Hit%20Result%20Structure%20%28by%20ref%29))
  (bind _teleportlocation (Variables|Default|GetTeleportLocation))
  (bind _asbp_first_person_character (Utilities|Casting|CastToBP_FirstPersonCharacter OtherActor))
  (Transformation|SetActorLocation _asbp_first_person_character (Transformation|GetWorldLocation _teleportlocation) false true)
  (Transformation|SetActorRotation _asbp_first_person_character (Transformation|GetWorldRotation _teleportlocation) true)
  (if (Variables|Default|GetChangeState)
    (Class|AkGameplayStatics|SetState 0 "Music_State_Group" (Utilities|String|StringToName (Variables|Default|GetStateName)))))

(event EventBeginPlay)

(event Collision|EventActorBeginOverlap
  (params (OtherActor :type Actor%20Object%20Reference)))

(event EventTick
  (params (DeltaSeconds :type Float%20%28single-precision%29))
  (bind _returnvalue (Game|GetPlayerCharacter 0))
  (bind _returnvalue_2 (Transformation|GetDistanceTo _returnvalue))
  (bind _returnvalue_3 (Math|Float|MapRangeClamped _returnvalue_2 1e+02 1.5e+03 1.2e+03 5e+01))
  (bind _returnvalue_4 (* DeltaSeconds _returnvalue_3))
  (bind _returnvalue_5 (Math|Rotator|MakeRotator 0.0 0.0 _returnvalue_4))
  (Transformation|AddLocalRotation (Variables|Default|GetSM_TeleportRotator) _returnvalue_5 false false)
  (Transformation|AddLocalRotation (Variables|Default|GetSM_TeleportRotatorCage2) (* _returnvalue_5 -1.2) false false))

(fn ConstructionScript)