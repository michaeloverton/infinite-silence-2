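; BP_InnerTunnel is a level geometry actor that animates a tunnel made of three independently rotating layers.
; Each tick, the inner, middle and outer rotator components add a local yaw rotation equal to their own speed variable multiplied by delta seconds, so the spin is frame-rate independent.
; It has no other logic; BeginPlay, overlap and the construction script are empty.
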(event EventBeginPlay)

(event Collision|EventActorBeginOverlap
  (params (OtherActor :type Actor%20Object%20Reference)))

(event EventTick
  (params (DeltaSeconds :type Float%20%28single-precision%29))
  (Transformation|AddLocalRotation (Variables|Default|GetInnerTunnelRotator) (Math|Rotator|MakeRotator 0.0 0.0 (* DeltaSeconds (Variables|Default|GetInnerRotationSpeed))) false false)
  (Transformation|AddLocalRotation (Variables|Default|GetMiddleTunnelRotator) (Math|Rotator|MakeRotator 0.0 0.0 (* DeltaSeconds (Variables|Default|GetMiddleRotationSpeed))) false false)
  (Transformation|AddLocalRotation (Variables|Default|GetOuterTunnelRotator) (Math|Rotator|MakeRotator 0.0 0.0 (* DeltaSeconds (Variables|Default|GetOuterRotationSpeed))) false false))

(fn ConstructionScript)