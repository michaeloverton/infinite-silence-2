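; Actor component that drives a Wwise RTPC from the distance between its owner and the first player character.
; Each tick, while that distance is under MaxDistance, it maps the range from MaxDistance to MinDistance onto RtpcStartPoint to RtpcEndpoint, clamped.
; The result is written to the RTPC named by ParamName; beyond MaxDistance no update is sent, so the last value remains.
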(event EventTick
  (params (DeltaSeconds :type Float%20%28single-precision%29))
  (bind _returnvalue (Components|GetOwner))
  (bind _returnvalue_2 (Game|GetPlayerCharacter 0))
  (bind _max_distance (Variables|Default|GetMax%20Distance))
  (bind _returnvalue_3 (Transformation|GetDistanceTo _returnvalue _returnvalue_2))
  (if (< _returnvalue_3 _max_distance)
    (Class|AkGameplayStatics|SetRTPCValue 0 (Math|Float|MapRangeClamped _returnvalue_3 _max_distance (Variables|Default|GetMin%20Distance) (Variables|Default|GetRtpcStartPoint) (Variables|Default|GetRtpcEndpoint)) 0 0 (Utilities|String|StringToName (Variables|Default|GetParamName)))))